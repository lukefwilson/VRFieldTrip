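; BPC_UpAndDown is an actor component that makes its owning actor bob vertically around its starting position.
; On InitializeComponent it caches the owner's location as OriginalLocation.
; Each Tick it sets the owner's location to that origin with a Z offset from a sine of game time, scaled by Speed and Height.
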(event EventTick
  (params (DeltaSeconds :type Float%20%28single-precision%29))
  (bind _originallocation (Variables|Default|GetOriginalLocation))
  (Transformation|SetActorLocation (Components|GetOwner) (Math|Vector|MakeVector (.x _originallocation) (.y _originallocation) (+ (.z _originallocation) (* (Math|Trig|Sin(Radians) (* (Utilities|Time|GetGameTimeinSeconds) (Variables|Default|GetSpeed))) (Variables|Default|GetHeight)))) false))

(event EventInitializeComponent
  (Variables|Default|SetOriginalLocation (Transformation|GetActorLocation (Components|GetOwner))))