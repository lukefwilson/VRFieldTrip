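; BP_GlobalScoreboard is an in-world scoreboard that shows one emissive text line per ClassroomChar actor, using that character's ScoreboardText.
; Two seconds after BeginPlay, it removes its placeholder text, spawns a stacked text render component for each character and stores them in an array.
; UpdateScores refreshes those lines by index and adds components for extra characters.
; Both paths rescale the background to the character count.
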(event Custom|UpdateScores
  (bind _outactors (Actor|GetAllActorsOfClass "/Game/Blueprints/ClassroomChar.ClassroomChar_C"))
  (for (_array_element _array_index) _outactors
    (if (> (Utilities|Array|Length (Variables|Default|GetTextComponents)) _array_index)
      (Rendering|Components|TextRender|SetText (Utilities|Array|Get(acopy) (Variables|Default|GetTextComponents) _array_index) (Variables|/Game/Blueprints/ClassroomChar.ClassroomChar_C|GetScoreboardText _array_element))
      (else
        (bind _returnvalue (AddComponent|AddTextRenderComponent false (Math|Transform|MakeTransform (Math|Vector|MakeVector 0.0 0.0 (+ (* _array_index (Variables|Default|GetLineHeight)) (Variables|Default|GetTopOffset))) "0, 0, 0" "1,1,1")))
        (Utilities|Array|Add (Variables|Default|GetTextComponents) _returnvalue)
        (Rendering|Components|TextRender|SetHorizontalAlignment _returnvalue "EHTA_Center")
        (Rendering|Components|TextRender|SetText _returnvalue (Variables|/Game/Blueprints/ClassroomChar.ClassroomChar_C|GetScoreboardText _array_element))
        (Rendering|Components|TextRender|SetWorldSize _returnvalue (Variables|Default|GetTextSize))
        (Class|TextRenderComponent|SetTextMaterial _returnvalue "/Game/Materials/M_EmissiveText.M_EmissiveText"))))
  (Transformation|SetRelativeScale3D (Variables|Default|GetBackground) (Math|Vector|MakeVector 0.5 2.0 (* (Utilities|Array|Length _outactors) -0.4))))

(event EventBeginPlay
  (Components|DestroyComponent (Variables|Default|GetTextRender))
  (Utilities|FlowControl|Delay 2.0)
  (bind _outactors (Actor|GetAllActorsOfClass "/Game/Blueprints/ClassroomChar.ClassroomChar_C"))
  (for (_array_element _array_index) _outactors
    (bind _returnvalue (AddComponent|AddTextRenderComponent false (Math|Transform|MakeTransform (Math|Vector|MakeVector 0.0 0.0 (+ (* _array_index (Variables|Default|GetLineHeight)) (Variables|Default|GetTopOffset))) "0, 0,0.000000" "1,1,1")))
    (Utilities|Array|Add (Variables|Default|GetTextComponents) _returnvalue)
    (Rendering|Components|TextRender|SetHorizontalAlignment _returnvalue "EHTA_Center")
    (Rendering|Components|TextRender|SetText _returnvalue (Variables|/Game/Blueprints/ClassroomChar.ClassroomChar_C|GetScoreboardText _array_element))
    (Rendering|Components|TextRender|SetWorldSize _returnvalue (Variables|Default|GetTextSize))
    (Class|TextRenderComponent|SetTextMaterial _returnvalue "/Game/Materials/M_EmissiveText.M_EmissiveText"))
  (Transformation|SetRelativeScale3D (Variables|Default|GetBackground) (Math|Vector|MakeVector 0.5 2.0 (* (Utilities|Array|Length _outactors) -0.4))))

(fn ConstructionScript)