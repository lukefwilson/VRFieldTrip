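; BP_Bacteria2 is a bacteria actor that players can highlight and tag, earning a point per hit until it becomes tagged after five.
; On BeginPlay it launches in a random direction with linear and angular physics velocity.
; Each tick it keeps a hit-count text above itself, facing the first player's pawn.
; RepNotify functions update that count and recolor the dynamic material orange once tagged, while the Highlighted notify is empty.
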(event EventBeginPlay
  (CallFunction|MovementBoost (Math|Random|RandomUnitVector)))

(event EventTick
  (params (DeltaSeconds :type Float%20%28single-precision%29))
  (Utilities|FlowControl|Sequence
    (:then_0
      (CallFunction|OrientScore))))

(event EventDestroyBacteria
  (Actor|DestroyActor))

(fn ConstructionScript
  (bind _returnvalue (Rendering|Material|CreateDynamicMaterialInstance 0 0 :!class /Script/Engine.PrimitiveComponent))
  (Variables|Default|SetDMI _returnvalue))

(fn OnRepHighlighted)

(fn OnRepTagged
  (if (Variables|Default|GetTagged)
    (Rendering|Material|SetVectorParameterValue (Variables|Default|GetDMI) "Color" "(R=1.000000,G=0.585369,B=0.000000,A=1.000000)" :!class /Script/Engine.MaterialInstanceDynamic)))

(fn OnRepTimesHit
  (Rendering|Components|TextRender|SetText (Variables|Default|GetHitCountText) (Utilities|String|BuildString(Integer) (Utilities|String|ToString(Integer) (Variables|Default|GetHitCount)) "/" 5)))

(fn MovementBoost
  (params (Direction :type Vector :default "0, 0, 0"))
  (bind _returnvalue (* Direction 2e+02))
  (Physics|SetPhysicsLinearVelocity _returnvalue false "None")
  (Class|PrimitiveComponent|SetPhysicsAngularVelocity _returnvalue false "None"))

(fn OrientScore
  (bind _returnvalue (Transformation|GetWorldLocation))
  (bind _hitcounttext (Variables|Default|GetHitCountText))
  (Transformation|SetWorldLocation (Variables|Default|GetHitCountText) (Math|Vector|MakeVector (.x _returnvalue) (.y _returnvalue) (+ (.z _returnvalue) 1e+02)) false)
  (Transformation|SetWorldRotation _hitcounttext (Math|Rotator|FindLookatRotation (Transformation|GetWorldLocation _hitcounttext) (Transformation|GetActorLocation (Game|Player|GetPlayerPawn 0))) false))

(fn Highlight
  (bind _output_get (Variables|Default|SetHighlighted (not (Variables|Default|GetHighlighted))))
  (return _output_get "NewEnumerator0"))

(fn Tag
  (params (TaggingActor :type Actor%20Object%20Reference))
  (Utilities|FlowControl|Sequence
    (:then_0
      (if (< (Variables|Default|GetHitCount) 5)
        (LocalVariables|SetPoints 1)
        (bind _output_get (Variables|Default|SetHitCount (+ (Variables|Default|GetHitCount) 1)))
        (if (>= _output_get 5)
          (Variables|Default|SetTagged true)))
      (return (LocalVariables|GetPoints)))))