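; BP_Bacteria_test2 is a test bacteria, kept in an UNUSED folder, that drifts as a gravity-free, physics-driven skeletal mesh.
; On BeginPlay it disables gravity and gives all bodies a random linear velocity, plus a random spin on one joint.
; Disconnected graphs hold unused experiments: per-joint impulses against gravity, a boost when motion stalls, a bounce on fast falls and a height cap.
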(event EventBeginPlay
  (bind _returnvalue (Math|Random|RandomUnitVector))
  (bind _returnvalue_2 (* _returnvalue 2e+02))
  (Physics|SetEnableGravity false)
  (Physics|SetEnableGravity (Variables|Default|GetSkeletalMesh) false)
  (Class|PrimitiveComponent|SetAllPhysicsLinearVelocity _returnvalue_2 false)
  (Class|PrimitiveComponent|SetPhysicsAngularVelocity _returnvalue_2 false "joint3"))

(event EventActorBeginOverlap
  (params (OtherActor :type Actor%20Object%20Reference)))

(event EventTick
  (params (DeltaSeconds :type Float%20%28single-precision%29)))

(fn ConstructionScript)