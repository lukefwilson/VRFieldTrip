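; BP_InfoPanel is an info panel actor that spawns and holds a model of either a bacterium or a red blood cell, chosen by InfoType.
; On BeginPlay it spawns the matching Blueprint, and AttachActor disables physics and collision on its primitive root before snapping it to ActorRoot.
; The spawned actor is kept as ChildInfoActor and destroyed along with the panel.
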(event EventDestroyed
  (Actor|DestroyActor (Variables|Default|GetChildInfoActor)))

(event EventBeginPlay
  (switch Utilities|FlowControl|Switch|SwitchonEnum_InfoType (Variables|Default|GetInfoType)
    (:NewEnumerator0
      (bind _returnvalue (Game|SpawnActorfromClass "/Game/Blueprints/UNUSED/BP_Bacteria.BP_Bacteria_C" (Math|Transform|MakeTransform "0, 0, 0" "0, 0, 0" "1,1,1") false 0))
      (CallFunction|AttachActor _returnvalue))
    (:NewEnumerator1
      (bind _returnvalue_2 (Game|SpawnActorfromClass "/Game/Blueprints/BP_RedBloodCell.BP_RedBloodCell_C" (Math|Transform|MakeTransform "0, 0, 0" "0, 0, 0" "1,1,1") false 0))
      (CallFunction|AttachActor _returnvalue_2))))

(fn ConstructionScript)

(fn AttachActor
  (params (Actor :type Actor%20Object%20Reference))
  (bind _asprimitive_component (Utilities|Casting|CastToPrimitiveComponent (VehicleSound|GetRootComponent Actor))
    (:then
      (Physics|SetSimulatePhysics _asprimitive_component false)
      (Collision|SetCollisionEnabled _asprimitive_component "NoCollision"))
    (:CastFailed
      _))
  (Class|Actor|AttachRootComponentto Actor (Variables|Default|GetActorRoot) "None" "SnapToTarget" true)
  (Variables|Default|SetChildInfoActor Actor))