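; Classroom pawn, named as unused, with mouse look, camera-relative movement and a reticle for highlighting or tagging actors.
; Tick places the reticle billboard by line trace and computes movement, applied through ServerMoveActor as an unswept relative offset on the root.
; Highlight and Tag inputs toggle the reticle on press and release.
; On release, a camera-forward trace passes the hit actor to Server-named events that call its HighlightMessage or TagMessage.
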(event Custom|ServerHighlightActor
  (params (Actor :type Actor%20Object%20Reference))
  (Class|BPIServerFunctions|Highlight(Message) Actor))

(event Custom|ServerTagActor
  (params (Actor :type Actor%20Object%20Reference))
  (Class|BPIServerFunctions|Tag(Message) Actor))

(event Custom|ServerMoveActor
  (params (ActorRootComponent :type Primitive%20Component%20Object%20Reference) (Velocity :type Vector :default "0, 0, 0"))
  (Transformation|AddRelativeLocation ActorRootComponent Velocity false))

(event EventTick
  (params (DeltaSeconds :type Float%20%28single-precision%29))
  (Utilities|FlowControl|Sequence
    (:then_0
      (CallFunction|UpdateReticle))
    (:then_1
      (|Movement))))

(event Input|ActionEvents|InputActionHighlight
  (bind _reticlebillboard (Variables|Default|GetReticleBillboard))
  (:Pressed
    (Rendering|SetVisibility _reticlebillboard (not (Variables|/Script/Engine.SceneComponent|GetbVisible _reticlebillboard)) false :!label _label))
  (:Released
    (Utilities|FlowControl|Sequence
      (:then_0
        (goto _label))
      (:then_1
        (bind (_hit _return) (CallFunction|StraightRayTrace))
        (if _return
          (CallFunction|ServerHighlightActor (.HitActor (Collision|BreakHitResult _hit))))))))

(event Input|ActionEvents|InputActionTag
  (bind _reticlebillboard (Variables|Default|GetReticleBillboard))
  (:Pressed
    (Rendering|SetVisibility _reticlebillboard (not (Variables|/Script/Engine.SceneComponent|GetbVisible _reticlebillboard)) false :!label _label))
  (:Released
    (Utilities|FlowControl|Sequence
      (:then_0
        (goto _label))
      (:then_1
        (bind (_hit _return) (CallFunction|StraightRayTrace))
        (if _return
          (CallFunction|ServerTagActor (.HitActor (Collision|BreakHitResult _hit))))))))

(event Input|AxisEvents|InputAxisTurn
  (params (AxisValue :type Float%20%28single-precision%29))
  ;[1 1 1] Turn with Mouse
  (Pawn|Input|AddControllerYawInput AxisValue))

(event Input|AxisEvents|InputAxisLookUp
  (params (AxisValue :type Float%20%28single-precision%29))
  ;[1 1 1] Lookup with Mouse (disabled in VR)
  (Pawn|Input|AddControllerPitchInput AxisValue))

(fn ConstructionScript)

(fn UpdateReticle
  (bind (_startpoint _endpoint) (Utilities|ReticlePoints))
  (bind _outhit (Collision|LineTraceByChannel _startpoint _endpoint "TraceTypeQuery1" false 0 "None"))
  (if true
    (LocalVariables|SetReticleLocation (.Location (Collision|BreakHitResult _outhit)))
    (else
      (LocalVariables|SetReticleLocation (.EndPoint (Utilities|ReticlePoints)))))
  (Transformation|SetWorldLocation (Variables|Default|GetReticleBillboard) (LocalVariables|GetReticleLocation) false))

(fn StraightRayTrace
  (bind _camera (Variables|Default|GetCamera))
  (bind _returnvalue (Transformation|GetWorldLocation _camera))
  (bind (_outhit _returnvalue_2) (Collision|LineTraceByChannel _returnvalue (+ _returnvalue (* (Math|Vector|GetForwardVector _camera) 5e+03)) "TraceTypeQuery1" false 0 "ForDuration"))
  (return _outhit _returnvalue_2))

(fn UpdateDebugText
  (Rendering|Components|TextRender|SetText (Variables|Default|GetDebugText) "Name - Score"))