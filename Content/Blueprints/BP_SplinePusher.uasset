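; Spline-following actor that starts moving along MovementSpline when play begins.
; On each update, the Pulse timeline's value, scaled by Speed, is added to an accumulated Distance, so the curve shapes velocity rather than position.
; The actor snaps to the spline's world location and rotation at that distance, with a quarter-turn yaw offset.
; The RunPulse event is an empty stub.
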(event Custom|RunPulse)

(event EventBeginPlay
  (bind _movementspline (Variables|Default|GetMovementSpline))
  (bind _data (Timeline|Pulse Play)
    (:Update
      (bind _output_get (Variables|Default|SetDistance (+ (Variables|Default|GetDistance) (* _data (Variables|Default|GetSpeed)))))
      (Transformation|SetActorLocationAndRotation (Class|SplineComponent|GetWorldLocationatDistanceAlongSpline _movementspline _output_get) (Math|Rotator|MakeRotator (.pitch (Class|SplineComponent|GetWorldRotationatDistanceAlongSpline _movementspline _output_get)) (+ (.yaw (Class|SplineComponent|GetWorldRotationatDistanceAlongSpline _movementspline _output_get)) 9e+01) (.roll (Class|SplineComponent|GetWorldRotationatDistanceAlongSpline _movementspline _output_get)))))))

(event EventActorBeginOverlap
  (params (OtherActor :type Actor%20Object%20Reference)))

(event EventTick
  (params (DeltaSeconds :type Float%20%28single-precision%29)))

(fn ConstructionScript)