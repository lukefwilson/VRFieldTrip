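; Physics-driven platelet actor that tumbles through the level and can be highlighted by other actors.
; BeginPlay sets random linear and angular velocity on the Body, which gets a dynamic material instance at construction.
; UpdateNearestSplinePosition caches the closest spline point, then destroys the actor if it is too far from the player.
; Highlight toggles a flag and returns an info type; Tag returns zero and the Highlighted OnRep is empty.
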(event EventBeginPlay
  (CallFunction|MovementBoost))

(event EventActorBeginOverlap
  (params (OtherActor :type Actor%20Object%20Reference)))

(event EventTick
  (params (DeltaSeconds :type Float%20%28single-precision%29)))

(fn ConstructionScript
  (bind _returnvalue (Rendering|Material|CreateDynamicMaterialInstance (Variables|Default|GetBody) 0 0 :!class /Script/Engine.PrimitiveComponent))
  (Variables|Default|SetDMI _returnvalue))

(fn OnRepHighlighted)

(fn MovementBoost
  (bind _returnvalue (Math|Random|RandomUnitVector))
  (bind _body (Variables|Default|GetBody))
  (bind _returnvalue_2 (* _returnvalue 2e+02))
  (Physics|SetPhysicsLinearVelocity _body _returnvalue_2 false "None")
  (Class|PrimitiveComponent|SetPhysicsAngularVelocity _body _returnvalue_2 false "None"))

(fn UpdateNearestSplinePosition
  (Utilities|FlowControl|Sequence
    (:then_0
      (for _array_element (Variables|/Game/Blueprints/BP_Spline.BP_Spline_C|GetSplinePositions (Variables|Default|GetSpline))
        (if (< (Math|Vector|VectorLength (- (Transformation|GetActorLocation) (.Location (Utilities|Struct|BreakStruct_VeinSplinePosition _array_element)))) (LocalVariables|GetClosestDistance))
          (LocalVariables|SetClosestSplinePosition _array_element)
          (LocalVariables|SetClosestDistance (Math|Vector|VectorLength (- (Transformation|GetActorLocation) (.Location (Utilities|Struct|BreakStruct_VeinSplinePosition _array_element)))))))
      (Variables|Default|SetNearestSplinePosition (LocalVariables|GetClosestSplinePosition)))
    (:then_1
      (CallFunction|SelfDestructifFar))))

(fn SelfDestructifFar
  (if (> (Math|Vector|VectorLength (- (Transformation|GetActorLocation (Game|Player|GetPlayerPawn 0)) (Transformation|GetActorLocation))) 7e+03)
    (Actor|DestroyActor)))

(fn Highlight
  (bind _output_get (Variables|Default|SetHighlighted (not (Variables|Default|GetHighlighted))))
  (return _output_get "NewEnumerator3"))

(fn Tag
  (params (TaggingActor :type Actor%20Object%20Reference))
  (return 0))