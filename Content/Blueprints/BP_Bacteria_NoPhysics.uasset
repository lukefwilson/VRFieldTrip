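; Non-physics bacteria actor that drifts at constant speed and can be highlighted or tagged for points.
; Tick moves the skeletal mesh along VelocityDirection without sweeping; the authority randomizes that direction at start and on overlaps, but steers toward CenterPoint after touching static mesh actors.
; Tag awards a point per hit up to five, then sets Tagged.
; RepNotifies update the hit counter text and recolor the dynamic material yellow once tagged.
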(event OnComponentBeginOverlap(Sphere)
  (params (OtherActor :type Actor%20Object%20Reference) (OtherComp :type Primitive%20Component%20Object%20Reference) (OtherBodyIndex :type Integer) (bFromSweep :type Boolean) (SweepResult :type Hit%20Result%20Structure%20%28by%20ref%29))
  ;[1 1 1] Change direction if hit something
  (Networking|SwitchHasAuthority
    (:Authority
      (if (Utilities|ClassIsChildOf (Utilities|GetClass OtherActor) "/Script/Engine.StaticMeshActor")
        (Variables|Default|SetVelocityDirection (Math|Vector|Normalize (- (Transformation|GetActorLocation (Variables|Default|GetCenterPoint)) (Transformation|GetActorLocation))))
        (else
          (Variables|Default|SetVelocityDirection (Math|Random|RandomUnitVector)))))))

(event EventDestroyBacteria
  ;[1 1 1] Destroy
  (Actor|DestroyActor))

(event EventBeginPlay
  (Networking|SwitchHasAuthority
    (:Authority
      (Variables|Default|SetVelocityDirection (Math|Random|RandomUnitVector)))))

(event EventTick
  (params (DeltaSeconds :type Float%20%28single-precision%29))
  (Utilities|FlowControl|Sequence
    (:then_0
      ;[1 1 1] Move in velocity direction
      (Variables|Default|SetDeltaSecs DeltaSeconds)
      (Variables|Default|SetCurrLocation (Transformation|GetWorldLocation (Variables|Default|GetSkeletalMesh)))
      (Transformation|SetWorldLocation (Variables|Default|GetSkeletalMesh) (+ (Variables|Default|GetCurrLocation) (* (Variables|Default|GetVelocityDirection) (* (Variables|Default|GetVelocityMag) (Variables|Default|GetDeltaSecs)))) false))))

(fn ConstructionScript
  (bind _returnvalue (Rendering|Material|CreateDynamicMaterialInstance 0 0 :!class /Script/Engine.PrimitiveComponent))
  (Variables|Default|SetDMI _returnvalue))

(fn OnRepVelocityDirection)

(fn OnRepHighlighted)

(fn OnRepTagged
  (if (Variables|Default|GetTagged)
    (Rendering|Material|SetVectorParameterValue (Variables|Default|GetDMI) "Color" "(R=0.755000,G=0.698637,B=0.000000,A=1.000000)" :!class /Script/Engine.MaterialInstanceDynamic)))

(fn OnRepHitCount
  (Rendering|Components|TextRender|SetText (Variables|Default|GetHitCountText) (Utilities|String|BuildString(Integer) (Utilities|String|ToString(Integer) (Variables|Default|GetHitCount)) "/" 5)))

(fn Highlight
  (bind _output_get (Variables|Default|SetHighlighted (not (Variables|Default|GetHighlighted))))
  (return _output_get "NewEnumerator0"))

(fn Tag
  (params (TaggingActor :type Actor%20Object%20Reference))
  (if (< (Variables|Default|GetHitCount) 5)
    (LocalVariables|SetPoints 1)
    (bind _output_get (Variables|Default|SetHitCount (+ (Variables|Default|GetHitCount) 1)))
    (if (>= _output_get 5)
      (Variables|Default|SetTagged true)))
  (return (LocalVariables|GetPoints)))