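; BP_ScoreAddition is a floating world-space popup that shows a "+N" score gain, then destroys itself.
; The construction script creates a dynamic material instance on the TextRender and sets its text from ScoreAddition.
; On BeginPlay, the Animation timeline raises the actor from its start, turns it toward the player pawn, scales the font and drives emissive strength from its Opacity track, destroying the actor when finished.
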(event EventBeginPlay
  (Variables|Default|SetStartingLocation (Transformation|GetActorLocation))
  (bind (_direction _opacity _height _fontsize) (Timeline|Animation Play)
    (:Update
      (Rendering|Material|SetScalarParameterValue (Variables|Default|GetDMI) "EmissiveStrength" (* _opacity 4.0) :!class /Script/Engine.MaterialInstanceDynamic)
      (Transformation|SetActorLocationAndRotation (Math|Vector|MakeVector (.x (Variables|Default|GetStartingLocation)) (.y (Variables|Default|GetStartingLocation)) (+ (.z (Variables|Default|GetStartingLocation)) (* _height 1e+02))) (Math|Rotator|FindLookatRotation (Transformation|GetActorLocation) (Transformation|GetActorLocation (Game|Player|GetPlayerPawn 0))))
      (Rendering|Components|TextRender|SetWorldSize (Variables|Default|GetTextRender) (* _fontsize 36.0)))
    (:Finished
      (Actor|DestroyActor))))

(event EventActorBeginOverlap
  (params (OtherActor :type Actor%20Object%20Reference)))

(event EventTick
  (params (DeltaSeconds :type Float%20%28single-precision%29)))

(fn ConstructionScript
  (bind _textrender (Variables|Default|GetTextRender))
  (bind _returnvalue (Rendering|Material|CreateDynamicMaterialInstance _textrender 0 0 :!class /Script/Engine.PrimitiveComponent))
  (Variables|Default|SetDMI _returnvalue)
  (Rendering|Components|TextRender|SetText _textrender (Utilities|String|BuildString(Integer) "" "+" (Variables|Default|GetScoreAddition))))