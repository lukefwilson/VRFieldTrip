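; Red blood cell actor that drifts off in a random direction under physics when play begins.
; MovementBoost sets the Body's linear velocity to a random fixed-speed vector twice, so the second call overrides the first.
; Construction stores a dynamic material instance of the Body, though nothing here changes it.
; Highlight toggles the Highlighted flag, whose OnRep is empty, and Tag is a stub returning zero.
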(event EventBeginPlay
  (CallFunction|MovementBoost))

(event EventActorBeginOverlap
  (params (OtherActor :type Actor%20Object%20Reference)))

(event EventTick
  (params (DeltaSeconds :type Float%20%28single-precision%29)))

(fn ConstructionScript
  (bind _returnvalue (Rendering|Material|CreateDynamicMaterialInstance (Variables|Default|GetBody) 0 0 :!class /Script/Engine.PrimitiveComponent))
  (Variables|Default|SetDMI _returnvalue))

(fn OnRepHighlighted)

(fn MovementBoost
  (bind _returnvalue (Math|Random|RandomUnitVector))
  (bind _body (Variables|Default|GetBody))
  (bind _returnvalue_2 (* _returnvalue 2e+02))
  (Physics|SetPhysicsLinearVelocity _body _returnvalue_2 false "None")
  (Physics|SetPhysicsLinearVelocity _body _returnvalue_2 false "None"))

(fn Highlight
  (bind _output_get (Variables|Default|SetHighlighted (not (Variables|Default|GetHighlighted))))
  (return _output_get))

(fn Tag
  (params (TaggingActor :type Actor%20Object%20Reference))
  (return 0))