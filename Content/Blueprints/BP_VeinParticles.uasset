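; BP_VeinParticles is a blood particle actor whose physics body is pushed in pulses along a vein-like flow.
; A Pulse timeline sets the body's linear velocity from the ClassroomChar player's nearest spline direction, scaled by curve value and MaxSpeed.
; UpdateOffset passes a position offset to the blood particle system.
; Highlight only toggles a flag, Tag is a stub, and the periodic spline-update timer is disconnected.
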(event Custom|UpdateOffset
  (params (NewPositionOffset :type Vector :default "0, 0, 0"))
  (Effects|Components|ParticleSystem|SetVectorParameter (Variables|Default|GetBloodParticles) "PositionOffset" NewPositionOffset))

(event EventBeginPlay
  (bind _asclassroom_char (Utilities|Casting|CastToClassroomChar (Game|Player|GetPlayerPawn 0)))
  (Variables|Default|SetPlayer _asclassroom_char)
  (bind _data (Timeline|Pulse Play)
    (:Update
      (if (> _data 0.0)
        (Physics|SetPhysicsLinearVelocity (Variables|Default|GetBody) (* (.Direction (Utilities|Struct|BreakStruct_VeinSplinePosition (Variables|/Game/Blueprints/ClassroomChar.ClassroomChar_C|GetNearestSplinePosition (Variables|Default|GetPlayer)))) (* _data (Variables|Default|GetMaxSpeed))) false "None")))))

(fn ConstructionScript
  (bind _returnvalue (Rendering|Material|CreateDynamicMaterialInstance (Variables|Default|GetBody) 0 0 :!class /Script/Engine.PrimitiveComponent))
  (Variables|Default|SetDMI _returnvalue))

(fn OnRepHighlighted)

(fn UpdateNearestSplinePosition
  (bind _asclassroom_char (Utilities|Casting|CastToClassroomChar (Game|Player|GetPlayerPawn 0)))
  (Variables|Default|SetNearestSplinePosition (Variables|/Game/Blueprints/ClassroomChar.ClassroomChar_C|GetNearestSplinePosition _asclassroom_char)))

(fn Tag
  (params (TaggingActor :type Actor%20Object%20Reference))
  (return 0))

(fn Highlight
  (bind _output_get (Variables|Default|SetHighlighted (not (Variables|Default|GetHighlighted))))
  (return _output_get "NewEnumerator1"))