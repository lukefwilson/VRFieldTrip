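; Red blood cell actor that drifts through a vein as a physics body, starting with a random push and spin.
; A two-second timer caches the nearest spline position and destroys the cell when far from the player.
; The Pulse timeline drives velocity along that position's direction, scaled by the pulse curve, or at constant speed when not pulsing.
; Highlight toggles a flag and returns an info type; Tag is a stub.
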(event EventBeginPlay
  (bind _nearestsplineposition (Variables|Default|GetNearestSplinePosition))
  (bind _direction (Utilities|Struct|BreakStruct_VeinSplinePosition _nearestsplineposition))
  (CallFunction|SetPlayer)
  (CallFunction|MovementBoost)
  (CallFunction|UpdateNearestSplinePosition)
  (Utilities|Time|SetTimerbyFunctionName 0 "UpdateNearestSplinePosition" 2.0 true)
  (bind _data (Timeline|Pulse Play)
    (:Update
      (if (Variables|Default|GetPulsing)
        (if (> _data 0.0)
          (Physics|SetPhysicsLinearVelocity (* _direction (* _data (Variables|Default|GetMaxSpeed))) false "None")
          (bind _returnvalue (Class|PrimitiveComponent|GetPhysicsAngularVelocity "None" :!label _label)))
        (else
          (Physics|SetPhysicsLinearVelocity (* _direction 3e+02) false "None")
          (goto _label))))))

(event EventActorBeginOverlap
  (params (OtherActor :type Actor%20Object%20Reference)))

(event EventTick
  (params (DeltaSeconds :type Float%20%28single-precision%29)))

(fn ConstructionScript
  (bind _returnvalue (Rendering|Material|CreateDynamicMaterialInstance (Variables|Default|GetBody) 0 0 :!class /Script/Engine.PrimitiveComponent))
  (Variables|Default|SetDMI _returnvalue))

(fn OnRepHighlighted)

(fn MovementBoost
  (bind _returnvalue (Math|Random|RandomUnitVector))
  (bind _body (Variables|Default|GetBody))
  (Physics|SetPhysicsLinearVelocity _body (* _returnvalue 5e+01) false "None")
  (Class|PrimitiveComponent|SetPhysicsAngularVelocity _body (* _returnvalue 4e+02) false "None"))

(fn UpdateNearestSplinePosition
  (Utilities|FlowControl|Sequence
    (:then_0
      (for _array_element (Variables|/Game/Blueprints/BP_Spline.BP_Spline_C|GetSplinePositions (Variables|Default|GetSpline))
        (if (< (Math|Vector|VectorLength (- (Transformation|GetActorLocation) (.Location (Utilities|Struct|BreakStruct_VeinSplinePosition _array_element)))) (LocalVariables|GetClosestDistance))
          (LocalVariables|SetClosestSplinePosition _array_element)
          (LocalVariables|SetClosestDistance (Math|Vector|VectorLength (- (Transformation|GetActorLocation) (.Location (Utilities|Struct|BreakStruct_VeinSplinePosition _array_element)))))))
      (Variables|Default|SetNearestSplinePosition (LocalVariables|GetClosestSplinePosition)))
    (:then_1
      (CallFunction|SelfDestructifFar))))

(fn SelfDestructifFar
  (Utilities|IsValid (Variables|Default|GetPlayer)
    (:Is%20Valid
      (if (> (Math|Vector|VectorLength (- (Transformation|GetActorLocation (Game|Player|GetPlayerPawn 0)) (Transformation|GetActorLocation))) 7e+03)
        (Actor|DestroyActor)))
    (:Is%20Not%20Valid
      (CallFunction|SetPlayer))))

(fn SetPlayer
  (bind _asclassroom_char (Utilities|Casting|CastToClassroomChar (Game|Player|GetPlayerPawn 0)))
  (Variables|Default|SetPlayer _asclassroom_char))

(fn Highlight
  (bind _output_get (Variables|Default|SetHighlighted (not (Variables|Default|GetHighlighted))))
  (return _output_get "NewEnumerator1"))

(fn Tag
  (params (TaggingActor :type Actor%20Object%20Reference))
  (return 0))