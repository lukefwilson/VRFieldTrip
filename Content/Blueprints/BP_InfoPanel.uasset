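; Info panel actor that displays a model of the blood or tissue entity selected by InfoType.
; BeginPlay spawns the matching Blueprint, mostly at reduced scale; white blood cell is only a placeholder print.
; AttachActor zeroes linear velocity, sets an angular spin, makes collision query-only, then snaps the model to ActorRoot.
; The spawned model is stored as ChildInfoActor and destroyed along with the panel.
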(event EventDestroyed
  (Actor|DestroyActor (Variables|Default|GetChildInfoActor)))

(event EventBeginPlay
  (switch Utilities|FlowControl|Switch|SwitchonEnum_InfoType (Variables|Default|GetInfoType)
    (:NewEnumerator0
      (bind _returnvalue (Game|SpawnActorfromClass "/Game/Blueprints/BP_Bacteria.BP_Bacteria_C" (Math|Transform|MakeTransform "0, 0, 0" "0, 0, 0" "1,1,1") true 0))
      (CallFunction|AttachActor _returnvalue))
    (:NewEnumerator1
      (bind _returnvalue_2 (Game|SpawnActorfromClass "/Game/Blueprints/BP_RedBloodCell.BP_RedBloodCell_C" (Math|Transform|MakeTransform "0, 0, 0" "0, 0, 0" "0.100000,0.100000,0.100000") true 0))
      (CallFunction|AttachActor _returnvalue_2)
      (Transformation|SetActorScale3D _returnvalue_2 "0.100000,0.100000,0.100000"))
    (:NewEnumerator2
      (bind _returnvalue_3 (Game|SpawnActorfromClass "/Game/Blueprints/BP_TissueCell.BP_TissueCell_C" (Math|Transform|MakeTransform "0, 0, 0" "0, 0, 0" "0.100000,0.100000,0.100000") true 0))
      (CallFunction|AttachActor _returnvalue_3))
    (:NewEnumerator3
      (bind _returnvalue_4 (Game|SpawnActorfromClass "/Game/Blueprints/BP_VeinPlatelet.BP_VeinPlatelet_C" (Math|Transform|MakeTransform "0, 0, 0" "0, 0, 0" "0.100000,0.100000,0.100000") true 0 0))
      (CallFunction|AttachActor _returnvalue_4)
      (Transformation|SetActorScale3D _returnvalue_4 "0.100000,0.100000,0.100000"))
    (:NewEnumerator4
      (Development|PrintString "Create new physics based actor for white blood cell"))))

(fn ConstructionScript)

(fn AttachActor
  (params (Actor :type Actor%20Object%20Reference))
  (bind _asprimitive_component (Utilities|Casting|CastToPrimitiveComponent (VehicleSound|GetRootComponent Actor))
    (:then
      (Physics|SetPhysicsLinearVelocity _asprimitive_component "0, 0, 0" false "None")
      (Class|PrimitiveComponent|SetPhysicsAngularVelocity _asprimitive_component "30.000000,0.000000,50.000000" false "None")
      (Collision|SetCollisionEnabled _asprimitive_component "QueryOnly"))
    (:CastFailed
      _))
  (Class|Actor|AttachRootComponentto Actor (Variables|Default|GetActorRoot) "None" "SnapToTarget" true)
  (Variables|Default|SetChildInfoActor Actor))