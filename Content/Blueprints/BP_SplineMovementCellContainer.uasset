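; BP_SplineMovementCellContainer is an actor that applies a repeating radial push through its ForwardRadialForce component.
; BeginPlay starts a looping one-second timer that calls Pulse, which fires the component's impulse.
; Tick and overlap events are empty, and leftover sine and cosine radius logic is never executed.
; Despite the name, the graphs contain no spline or movement logic.
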(event EventBeginPlay
  (Utilities|Time|SetTimerbyFunctionName 0 "Pulse" 1.0 true))

(event EventActorBeginOverlap
  (params (OtherActor :type Actor%20Object%20Reference)))

(event EventTick
  (params (DeltaSeconds :type Float%20%28single-precision%29)))

(fn ConstructionScript)

(fn Pulse
  (Class|RadialForceComponent|FireImpulse (Variables|Default|GetForwardRadialForce)))