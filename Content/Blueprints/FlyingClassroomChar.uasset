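; Networked player character for a flying classroom that highlights and tags actors it aims at.
; Tick moves a reticle billboard via a visibility trace; Highlight and Tag inputs toggle it and, on release, trace from the camera and call server events.
; Highlighting replicates the target, whose OnRep spawns an info panel facing the local player's pawn.
; Tagging adds the target's returned value to a replicated Score shown in the player text.
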(event Custom|ServerSetName
  (params (name :type String))
  ;[1 1 1] Run on Server Actions
  (Variables|Default|SetName "None"))

(event Custom|ServerSetTeacher
  (params (Teacher :type Boolean :default false))
  ;[1 1 1] Run on Server Actions
  (Variables|Default|SetTeacher Teacher))

(event Custom|ServerHighlightActor
  (params (Actor :type Actor%20Object%20Reference))
  ;[1 1 1] Run on Server Actions
  (bind _highlighted (Class|BPIServerFunctions|Highlight(Message) Actor))
  (if _highlighted
    (Variables|Default|SetHighlightedActor Actor)
    (else
      (Variables|Default|SetHighlightedActor 0))))

(event Custom|ServerTagActor
  (params (Actor :type Actor%20Object%20Reference))
  ;[1 1 1] Run on Server Actions
  (bind _pointincrease (Class|BPIServerFunctions|Tag(Message) Actor self))
  (CallFunction|AddtoScore _pointincrease))

(event EventBeginPlay
  ;[1 1 1] ???
  (bind _asnetworked_game_instance (Utilities|Casting|CastToNetworkedGameInstance (Game|GetGameInstance)))
  (if (Variables|/Game/Blueprints/NetworkedGameInstance.NetworkedGameInstance_C|GetTeacher _asnetworked_game_instance)
    _))

(event EventActorBeginOverlap
  (params (OtherActor :type Actor%20Object%20Reference)))

(event EventTick
  (params (DeltaSeconds :type Float%20%28single-precision%29))
  ;[1 1 1] Update Reticle
  (CallFunction|UpdateReticle))

(event Input|ActionEvents|InputActionHighlight
  (bind _reticlebillboard (Variables|Default|GetReticleBillboard))
  ;[1 1 1] Interactions
  ;;[1 1 1] Highlight action
  (:Pressed
    (Rendering|SetVisibility _reticlebillboard (not (Variables|/Script/Engine.SceneComponent|GetbVisible _reticlebillboard)) false :!label _label))
  (:Released
    (Utilities|FlowControl|Sequence
      (:then_0
        (goto _label))
      (:then_1
        (bind (_hit _return) (CallFunction|StraightRayTrace))
        (if _return
          (CallFunction|ServerHighlightActor (.HitActor (Collision|BreakHitResult _hit))))))))

(event Input|ActionEvents|InputActionTag
  (bind _reticlebillboard (Variables|Default|GetReticleBillboard))
  ;[1 1 1] Interactions
  ;;[1 1 1] Tag action
  (:Pressed
    (Rendering|SetVisibility _reticlebillboard (not (Variables|/Script/Engine.SceneComponent|GetbVisible _reticlebillboard)) false :!label _label))
  (:Released
    (Utilities|FlowControl|Sequence
      (:then_0
        (goto _label))
      (:then_1
        (bind (_hit _return) (CallFunction|StraightRayTrace))
        (if _return
          (CallFunction|ServerTagActor (.HitActor (Collision|BreakHitResult _hit))))))))

(event Input|AxisEvents|InputAxisLookUp
  (params (AxisValue :type Float%20%28single-precision%29)))

(fn ConstructionScript)

(fn UpdateReticle
  (bind (_startpoint _endpoint) (Utilities|ReticlePoints))
  (bind _outhit (Collision|LineTraceByChannel _startpoint _endpoint "TraceTypeQuery1" false 0 "None"))
  (if true
    (LocalVariables|SetReticleLocation (.Location (Collision|BreakHitResult _outhit)))
    (else
      (LocalVariables|SetReticleLocation "0, 0, 0")))
  (Transformation|SetWorldLocation (Variables|Default|GetReticleBillboard) (LocalVariables|GetReticleLocation) false))

(fn StraightRayTrace
  (bind _camera (Variables|Default|GetCamera))
  (bind _returnvalue (Transformation|GetWorldLocation _camera))
  (bind (_outhit _returnvalue_2) (Collision|LineTraceByChannel _returnvalue (+ _returnvalue (* (Math|Vector|GetForwardVector _camera) 5e+03)) "TraceTypeQuery1" false 0 "None"))
  (return _outhit _returnvalue_2))

(fn AddtoScore
  (params (Addition :type Integer :default 0))
  (Variables|Default|SetScore (+ (Variables|Default|GetScore) Addition)))

(fn OnRepHighlightedActor
  ;[1 1 1] Create info panel in front of local character
  (bind _asflying_classroom_char (Utilities|Casting|CastToFlyingClassroomChar (Game|Player|GetPlayerPawn 0)))
  (Utilities|IsValid (Variables|FlyingClassroomChar_C|GetInfoPanel _asflying_classroom_char)
    (:Is%20Valid
      (Actor|DestroyActor (Variables|FlyingClassroomChar_C|GetInfoPanel _asflying_classroom_char)))
    (:Is%20Not%20Valid
      _))
  (Utilities|IsValid (Variables|Default|GetHighlightedActor)
    (:Is%20Valid
      (bind _returnvalue (Game|SpawnActorfromClass "/Game/Blueprints/BP_InfoPanel.BP_InfoPanel_C" (Math|Transform|MakeTransform (+ (.location (Transformation|GetActorTransform _asflying_classroom_char)) (* (Math|Vector|GetForwardVector (Variables|FlyingClassroomChar_C|GetCamera _asflying_classroom_char)) 4e+02)) (Math|Rotator|FindLookatRotation (+ (.location (Transformation|GetActorTransform _asflying_classroom_char)) (* (Math|Vector|GetForwardVector (Variables|FlyingClassroomChar_C|GetCamera _asflying_classroom_char)) 4e+02)) (.location (Transformation|GetActorTransform _asflying_classroom_char))) "1,1,1") false 0))
      (Variables|FlyingClassroomChar_C|SetInfoPanel _asflying_classroom_char _returnvalue)
      (Variables|FlyingClassroomChar_C|SetHighlightedActor _asflying_classroom_char (Variables|Default|GetHighlightedActor)))))

(fn OnRepScore
  (CallFunction|UpdatePlayerText))

(fn OnRepName
  (CallFunction|UpdatePlayerText))

(fn OnRepTeacher)

(fn UpdatePlayerText
  (Rendering|Components|TextRender|SetText (Variables|Default|GetPlayerText) (Utilities|String|BuildString(Integer) "" " - " (Variables|Default|GetScore))))