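; Construction-script generator that scatters child actors as tissue cells over surrounding WorldStatic geometry; event graph is empty.
; Nested loops, both sized by NumCellsPerLoop, fire long line traces from the actor at evenly stepped yaw and random pitch.
; Each hit adds a child actor at the impact location with random displacement and per-axis scale, attached to Root keeping world position.
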(event EventBeginPlay)

(event EventActorBeginOverlap
  (params (OtherActor :type Actor%20Object%20Reference)))

(event EventTick
  (params (DeltaSeconds :type Float%20%28single-precision%29)))

(fn ConstructionScript
  (bind _scalemin (Variables|Default|GetScaleMin))
  (bind _scalemax (Variables|Default|GetScaleMax))
  (bind _returnvalue (Math|Random|RandomFloatinRange _scalemin _scalemax))
  (for _index (range 1 (Variables|Default|GetNumCellsPerLoop))
    (for _index_2 (range 1 (Variables|Default|GetNumCellsPerLoop))
      (bind (_outhit _returnvalue_2) (Collision|LineTraceForObjects (Transformation|GetActorLocation) (Math|Vector|RotateVector (+ (Transformation|GetActorLocation) "10000000.000000, 0, 0") (Math|Rotator|MakeRotator (Math|Conversions|ToFloat(Integer) (Math|Random|RandomIntegerinRange 0 360)) (Math|Conversions|ToFloat(Integer) (* _index (/ 360 (Variables|Default|GetNumCellsPerLoop)))) 0.0)) (Utilities|Array|MakeArray "ObjectTypeQuery1") false 0 "None"))
      (if _returnvalue_2
        (bind _returnvalue_3 (AddComponent|AddChildActorComponent true (Math|Transform|MakeTransform (+ (.Location (Collision|BreakHitResult _outhit)) (* (Math|Random|RandomUnitVector) (Math|Random|RandomFloatinRange (Variables|Default|GetDisplacementMin) (Variables|Default|GetDisplacementMax)))) "0, 0, 0" (Math|Vector|MakeVector _returnvalue _returnvalue _returnvalue))))
        (Class|SceneComponent|Attachto _returnvalue_3 (Variables|Default|GetRoot) "None" "KeepWorldPosition" true)))))