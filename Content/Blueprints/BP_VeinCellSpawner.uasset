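; Blood vein cell spawner that continuously emits small red blood cell and platelet actors at randomized positions around itself and hands each a spline.
; BeginPlay starts two self-recalling events, each looping through a random Delay of up to a second.
; Both loops share SpawnCount and NextSpline, using modulo checks after each spawn to switch the next cell of either type between MainSpline and OffshootSpline.
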(event Custom|SpawnPlatelet
  (bind _returnvalue (Transformation|GetActorLocation))
  (Utilities|FlowControl|Delay (Math|Random|RandomFloatinRange 0.1 1.0))
  (Variables|Default|SetSpawnCount (+ (Variables|Default|GetSpawnCount) 1))
  (Game|SpawnActorfromClass "/Game/Blueprints/BP_VeinPlatelet.BP_VeinPlatelet_C" (Math|Transform|MakeTransform (Math|Vector|MakeVector (+ (.x _returnvalue) (Math|Random|RandomFloatinRange -2e+02 2e+02)) (.y _returnvalue) (+ (.z _returnvalue) (Math|Random|RandomFloatinRange -2e+02 2e+02))) "0, 0, 0" "0.100000,0.100000,0.100000") false (Variables|Default|GetNextSpline) 0)
  (CallFunction|SpawnPlatelet)
  (if (== (Math|Integer|%(Integer) (Variables|Default|GetSpawnCount) 3) 0)
    (Variables|Default|SetNextSpline (Variables|Default|GetOffshootSpline))
    (else
      (Variables|Default|SetNextSpline (Variables|Default|GetMainSpline)))))

(event Custom|SpawnRedBloodCell
  (bind _returnvalue (Transformation|GetActorLocation))
  (Utilities|FlowControl|Delay (Math|Random|RandomFloatinRange 0.1 1.0))
  (Variables|Default|SetSpawnCount (+ (Variables|Default|GetSpawnCount) 1))
  (Game|SpawnActorfromClass "/Game/Blueprints/BP_VeinRedBloodCell.BP_VeinRedBloodCell_C" (Math|Transform|MakeTransform (Math|Vector|MakeVector (+ (.x _returnvalue) (Math|Random|RandomFloatinRange -2e+02 2e+02)) (.y _returnvalue) (+ (.z _returnvalue) (Math|Random|RandomFloatinRange -2e+02 2e+02))) "0, 0, 0" "0.100000,0.100000,0.100000") false (Variables|Default|GetNextSpline) 0)
  (CallFunction|SpawnRedBloodCell)
  (if (== (Math|Integer|%(Integer) (Variables|Default|GetSpawnCount) 2) 0)
    (Variables|Default|SetNextSpline (Variables|Default|GetMainSpline))
    (else
      (Variables|Default|SetNextSpline (Variables|Default|GetOffshootSpline)))))

(event EventBeginPlay
  (Variables|Default|SetNextSpline (Variables|Default|GetMainSpline))
  (CallFunction|SpawnRedBloodCell)
  (CallFunction|SpawnPlatelet))

(fn ConstructionScript)